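; FPS player controller Blueprint that shows the end-of-mission screens.
; Mission completion adds the won widget to the viewport, then casts the game mode with nothing following.
; Mission failure switches on authority to call Multy directly or through Server, and Multy adds a widget with no class shown.
; Setting the game mode's Won flag and blending to a finish camera are disconnected.
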(event `self.OnMissionCompleted`
  (params (InstigatorPawn :type "Pawn Object Reference"))
  (bind _returnvalue (`|CreateWidget` "/Game/UI/WBP_GameOver_Won.WBP_GameOver_Won_C"))
  (`UserWidget.AddToViewport` _returnvalue 0)
  (bind _asbp_game_mode (cast `/Game/Blueprints/BP_GameMode` (`GameplayStatics.GetGameMode`))))

(event `Mission Faild`
  (`/Engine/EditorBlueprintResources/ActorMacros.Switch Has Authority`
    (:`Authority`
      (`self.multy`))
    (:`Remote`
      (`self.server`))))

(event `multy`
  (bind _returnvalue (`|CreateWidget` "/Game/UI/WBP_GameOver_Faild.WBP_GameOver_Faild_C"))
  (`UserWidget.AddToViewport` _returnvalue 0))

(event `server`
  (`self.multy`))

(fn `UserConstructionScript`)